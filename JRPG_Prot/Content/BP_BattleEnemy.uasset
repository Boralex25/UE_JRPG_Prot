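; BP_BattleEnemy is a battle enemy actor that displays its health and damage numbers.
; UpdateHP sets the progress bar in its WBP_EnemyHP widget component from current over max HP, and runs on BeginPlay.
; ShowDamageNumber spawns a BP_DamageNumber actor at an offset above the enemy, passing the damage, with debug prints.
; BeginPlay also creates a WBP_DamageNumber widget, but the logic placing it in the viewport is unconnected.
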(event Custom|ShowDamageNumber
  (params (Damage :type Integer))
  (bind _returnvalue (Transformation|GetActorLocation))
  (Development|PrintString "Hello" true true "(R=0.000000,G=0.000000,B=0.000000,A=1.000000)")
  (Game|SpawnActorfromClass "/Game/BP_DamageNumber.BP_DamageNumber_C" (Math|Transform|MakeTransform (Math|Vector|MakeVector (- (.x _returnvalue) 6e+01) (.y _returnvalue) (+ (.z _returnvalue) 9e+01)) "0, 0, 0" "1.000000,1.000000,1.000000") "Undefined" "MultiplyWithRoot" 0 Damage 0)
  (Development|PrintString "SPAWN DMG NMB" true true "(R=1.000000,G=0.135481,B=0.000000,A=1.000000)"))

(event EventBeginPlay
  (CallFunction|UpdateHP)
  (bind _returnvalue (UserInterface|CreateWidget "/Game/WBP_DamageNumber.WBP_DamageNumber_C"))
  (Variables|Default|SetWBP_DamageNumber _returnvalue))

(event Collision|EventActorBeginOverlap
  (params (OtherActor :type Actor%20Object%20Reference)))

(event EventTick
  (params (DeltaSeconds :type Float%20%28single-precision%29)))

(fn ConstructionScript)

(fn UpdateHP
  (Development|PrintString "UPDATE ENEMY HP" true true "(R=0.137269,G=0.000000,B=1.000000,A=1.000000)")
  (bind _aswbp_enemy_hp (Utilities|Casting|CastToWBP_EnemyHP (UserInterface|GetUserWidgetObject (Variables|Default|GetHP_Widget))))
  (Progress|SetPercent (Variables|/Game/WBP_EnemyHP.WBP_EnemyHP_C|GetProgressBar_0 _aswbp_enemy_hp) (/ (Variables|Default|GetCurrentHP) (Variables|Default|GetMaxHP))))