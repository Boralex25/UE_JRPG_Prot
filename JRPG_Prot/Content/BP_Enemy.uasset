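; BP_Enemy is an enemy that starts a battle when the player character enters its detection sphere.
; On overlap it sets the PlayerDetected blackboard key, stops its AI movement and brain logic, moves the player to BattleSpawnPoint, locks player movement and calls StartBattle on BP_BattleManager.
; A MoveToNextPoint event loops through PatrolPoints with AIMoveTo, but nothing in this Blueprint calls it.
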(event OnComponentBeginOverlap(DetectionSphere)
  (params (OverlappedComponent :type Primitive%20Component%20Object%20Reference) (OtherActor :type Actor%20Object%20Reference) (OtherComp :type Primitive%20Component%20Object%20Reference) (OtherBodyIndex :type Integer) (bFromSweep :type Boolean) (SweepResult :type Hit%20Result%20Structure%20%28by%20ref%29))
  (bind _self self)
  (bind _returnvalue (AI|GetAIController _self))
  (Utilities|Casting|CastToBP_ThirdPersonCharacter OtherActor)
  (AI|Components|Blackboard|SetValueasBool (AI|GetBlackboard _returnvalue) (Utilities|Name|MakeLiteralName "PlayerDetected") true)
  (AI|Navigation|StopMovement _returnvalue)
  (bind _asbp_enemy_controller (Utilities|Casting|CastToBP_EnemyController _returnvalue))
  (AI|Logic|StopLogic (Variables|/Script/AIModule.AIController|GetBrainComponent _asbp_enemy_controller) "")
  (bind _asbp_third_person_character (Utilities|Casting|CastToBP_ThirdPersonCharacter OtherActor))
  (Transformation|SetActorLocation _asbp_third_person_character (Transformation|GetActorLocation (Variables|Default|GetBattleSpawnPoint)) false false)
  (Variables|Default|SetIsBattleStarted true)
  (bind _returnvalue_2 (Actor|GetActorOfClass "/Game/BP_BattleManager.BP_BattleManager_C"))
  (Variables|Default|SetBattleManagerRef _returnvalue_2)
  (Variables|/Game/ThirdPerson/Blueprints/BP_ThirdPersonCharacter.BP_ThirdPersonCharacter_C|SetCanMove _asbp_third_person_character false)
  (Default|StartBattle (Variables|Default|GetBattleManagerRef)))

(event Custom|MoveToNextPoint
  (AI|AIMoveTo self "0, 0, 0" (Utilities|Array|Get(acopy) (Variables|Default|GetPatrolPoints) (Variables|Default|GetCurrentPointIndex)) 1.0 false
    (:OnSuccess
      (Development|PrintString "Hello")
      (Variables|Default|SetCurrentPointIndex (Math|Integer|%(Integer) (+ (Variables|Default|GetCurrentPointIndex) 1) (Utilities|Array|Length (Variables|Default|GetPatrolPoints))))
      (CallFunction|MovetoNextPoint))))

(event EventBeginPlay)

(event Collision|EventActorBeginOverlap
  (params (OtherActor :type Actor%20Object%20Reference)))

(fn ConstructionScript)