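; BP_DamageNumber is an actor that displays a damage value through a WBP_DamageNumber widget held in its DamageWidget component.
; On BeginPlay it casts the component's widget and copies its Damage into the widget's DamageValue.
; SetDamage performs the same cast before passing a damage value on through a SetDamage call.
; A timeline that would move the actor upward and destroy it, plus a debug print, is left unconnected and never runs.
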(event EventBeginPlay
  (bind _aswbp_damage_number (Utilities|Casting|CastToWBP_DamageNumber (UserInterface|GetUserWidgetObject (Variables|Default|GetDamageWidget))))
  (Variables|/Game/WBP_DamageNumber.WBP_DamageNumber_C|SetDamageValue _aswbp_damage_number (Variables|Default|GetDamage)))

(fn ConstructionScript)

(fn SetDamage
  (params (Damage :type Integer))
  (Utilities|Casting|CastToWBP_DamageNumber (UserInterface|GetUserWidgetObject (Variables|Default|GetDamageWidget)))
  (CallFunction|SetDamage Damage))